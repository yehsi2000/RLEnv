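; Prey character that eats grass and takes damage, with Health and Hunger restored on Reset.
; Capsule overlaps track the touched grass, and Tick refills Hunger when it is close, with a timer as eating cooldown.
; See builds an observation from capped inverse absolute X/Y distances to the AI controller's Predator and Grass, zeroed when either is missing.
; The game mode registration code is disconnected and never runs.
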(event `self.ReceiveBeginPlay`
  (`parent.ReceiveBeginPlay`)
  (`|ExecutionSequence`
    (:`then_0`
      (bind _asbp_prey_aicontroller (cast `/Game/Blueprints/Controller/BP_PreyAIController` (`self.GetController`)))
      (set `self.AIControl` _asbp_prey_aicontroller))))

(event `self.ReceiveTick`
  (params (DeltaSeconds :type "Float (single-precision)"))
  (bind _touchinggrass (`self.TouchingGrass`))
  (`parent.ReceiveTick` DeltaSeconds)
  (`/Engine/EditorBlueprintResources/StandardMacros.IsValid` (`self.AIControl`)
    (:`Is Valid`
      (if (`self.CanEat`)
        (`/Engine/EditorBlueprintResources/StandardMacros.IsValid` _touchinggrass
          (:`Is Valid`
            (if (< (`KismetMathLibrary.Vector_Distance` (`self.K2_GetActorLocation`) (`self.K2_GetActorLocation` _touchinggrass)) 150.0)
              (set `self.Hunger` (`KismetMathLibrary.FMin` (+ (`self.Hunger`) 20.0) 100.0))
              (set `self.isHungry` false)
              (set `self.CanEat` false)
              (`KismetSystemLibrary.K2_SetTimerDelegate` (delegate `Can eat`) 1.0))))))))

(event `Can eat`
  (set `self.CanEat` true))

(event `self.ReceiveAnyDamage`
  (params (Damage :type "Float (single-precision)") (DamageType :type "DamageType Object Reference") (InstigatedBy :type "Controller Object Reference") (DamageCauser :type "Actor Object Reference"))
  (bind _output_get (set `self.Health` (- (`self.Health`) Damage)))
  (`KismetSystemLibrary.PrintString` (`KismetTextLibrary.Conv_TextToString` (`|FormatText` "Damged, HP={hp}" _output_get))))

(event `self.Reset`
  (`parent.Reset`)
  (set `self.Health` 100.0)
  (set `self.Hunger` 100.0))

(event `self.CapsuleComponent.OnComponentBeginOverlap`
  (params (OverlappedComponent :type "PrimitiveComponent Object Reference") (OtherActor :type "Actor Object Reference") (OtherComp :type "PrimitiveComponent Object Reference") (OtherBodyIndex :type Integer) (bFromSweep :type Boolean) (SweepResult :type "HitResult Structure (by ref)"))
  (`KismetSystemLibrary.PrintString` "begin overlap")
  (bind _asbp_grass (cast `/Game/Blueprints/Environment/BP_Grass` OtherActor))
  (set `self.TouchingGrass` _asbp_grass))

(event `self.CapsuleComponent.OnComponentEndOverlap`
  (params (OverlappedComponent :type "PrimitiveComponent Object Reference") (OtherActor :type "Actor Object Reference") (OtherComp :type "PrimitiveComponent Object Reference") (OtherBodyIndex :type Integer))
  (`KismetSystemLibrary.PrintString` "end overlap")
  (cast `/Game/Blueprints/Environment/BP_Grass` OtherActor)
  (set `self.TouchingGrass` null))

(fn `See`
  (returns (ReturnValue :type "Array of Vector2D Structure"))
  (locals (Ret :type "Array of Vector2D Structure"))
  (bind _ret (`local.Ret`))
  (bind _ret_2 (`local.Ret`))
  (bind _predator (`/Game/Blueprints/Controller/BP_PreyAIController.Predator` (`self.AIControl`)))
  (bind _grass (`/Game/Blueprints/Controller/BP_PreyAIController.Grass` (`self.AIControl`)))
  (bind (_returnvalue_x _returnvalue_y) (`KismetMathLibrary.BreakVector` (- (`self.K2_GetActorLocation` _grass) (`self.K2_GetActorLocation`))))
  (bind (_returnvalue_x_2 _returnvalue_y_2) (`KismetMathLibrary.BreakVector` (- (`self.K2_GetActorLocation` _predator) (`self.K2_GetActorLocation`))))
  (`KismetArrayLibrary.Array_Clear` (`local.Ret`))
  (`/Engine/EditorBlueprintResources/StandardMacros.IsValid` (`self.AIControl`)
    (:`Is Valid`
      (`/Engine/EditorBlueprintResources/StandardMacros.IsValid` _predator
        (:`Is Valid`
          (`KismetArrayLibrary.Array_Add` _ret_2 (`KismetMathLibrary.MakeVector2D` (`KismetMathLibrary.FMin` (/ 1.0 (+ (`KismetMathLibrary.Abs` _returnvalue_x_2) 0.1)) (`self.Max`)) (`KismetMathLibrary.FMin` (/ 1.0 (+ (`KismetMathLibrary.Abs` _returnvalue_y_2) 0.1)) (`self.Max`)))))
        (:`Is Not Valid`
          (`KismetArrayLibrary.Array_Add` _ret_2 (0.0 0.0))))
      (`/Engine/EditorBlueprintResources/StandardMacros.IsValid` _grass
        (:`Is Valid`
          (`KismetArrayLibrary.Array_Add` _ret (`KismetMathLibrary.MakeVector2D` (`KismetMathLibrary.FMin` (/ 1.0 (+ (`KismetMathLibrary.Abs` _returnvalue_x) 0.1)) (`self.Max`)) (`KismetMathLibrary.FMin` (/ 1.0 (+ (`KismetMathLibrary.Abs` _returnvalue_y) 0.1)) (`self.Max`)))))
        (:`Is Not Valid`
          (`KismetArrayLibrary.Array_Add` _ret (0.0 0.0))))
      (return (`local.Ret`)))
    (:`Is Not Valid`
      (return (`local.Ret`)))))

(fn `UserConstructionScript`
  (`parent.UserConstructionScript`))