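; Game mode for a predator-prey environment, apparently for reinforcement learning, that provides a reset of both agents.
; ResetFunction destroys the Predator and Prey if valid, then spawns replacements at their stored initial transforms and gives each its default controller.
; The function does not assign the new actors back to the Predator and Prey variables.
; BeginPlay, Tick and the construction script are empty.
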(event `self.ReceiveTick`
  (params (DeltaSeconds :type "Float (single-precision)")))

(fn `ResetFunction`
  (bind _prey (`self.Prey`))
  (`|ExecutionSequence`
    (:`then_0`
      (`/Engine/EditorBlueprintResources/StandardMacros.IsValid` (`self.Predator`)
        (:`Is Valid`
          (`self.K2_DestroyActor` (`self.Predator`))
          (bind _returnvalue (`|SpawnActorFromClass` "/Game/Blueprints/Character/BP_Predator.BP_Predator_C" (`self.InitPredatorTrans`) "AdjustIfPossibleButAlwaysSpawn" "MultiplyWithRoot" null null))
          (`Pawn.SpawnDefaultController` _returnvalue))))
    (:`then_1`
      (`/Engine/EditorBlueprintResources/StandardMacros.IsValid` _prey
        (:`Is Valid`
          (`self.K2_DestroyActor` _prey)
          (bind _returnvalue_2 (`|SpawnActorFromClass` "/Game/Blueprints/Character/BP_Prey.BP_Prey_C" (`self.InitPreyTrans`) "AdjustIfPossibleButAlwaysSpawn" "MultiplyWithRoot" null null))
          (`Pawn.SpawnDefaultController` _returnvalue_2))))))

(fn `UserConstructionScript`)