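; AI controller for a predator that runs the BT_Predator behavior tree and hunts BP_Prey actors by sight.
; Sight perception sets the blackboard TargetActor, or clears it and records LastLocation when the prey is lost.
; Tick damages the target directly when it is within close range, then a one-shot timer enforces a short attack cooldown.
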(event `self.ReceiveBeginPlay`
  (`parent.ReceiveBeginPlay`)
  (`self.RunBehaviorTree` "/Game/Blueprints/AI/BT_Predator.BT_Predator"))

(event `self.AIPerception.OnTargetPerceptionUpdated`
  (params (Actor :type "Actor Object Reference") (Stimulus :type "AIStimulus Structure"))
  (bind _returnvalue (`AIPerceptionSystem.GetSenseClassForStimulus` Stimulus))
  (if (== _returnvalue "/Script/AIModule.AISense_Sight")
    (`self.HandleSightSense` Actor Stimulus)))

(event `self.ReceiveTick`
  (params (DeltaSeconds :type "Float (single-precision)"))
  (`parent.ReceiveTick` DeltaSeconds)
  (if (`self.bCanAttack`)
    (bind _asactor (cast `Actor` (`BlackboardComponent.GetValueAsObject` (`self.Blackboard`) "TargetActor")))
    (if (< (`KismetMathLibrary.Vector_Distance` (`self.K2_GetActorLocation` (`self.K2_GetPawn`)) (`self.K2_GetActorLocation` _asactor)) 150.0)
      (`GameplayStatics.ApplyDamage` _asactor 50.0 null null "/Script/Engine.DamageType")
      (set `self.bCanAttack` false)
      (`KismetSystemLibrary.K2_SetTimerDelegate` (delegate `Can Attack Again`) 1.0))))

(event `Can Attack Again`
  (set `self.bCanAttack` true))

(fn `HandleSightSense`
  (params (SenseActor :type "Actor Object Reference") (Stimulus :type "AIStimulus Structure"))
  (bind (_age _expirationage _strength _stimuluslocation _receiverlocation _tag _bsuccessfullysensed) (break `AIStimulus` Stimulus))
  (bind _asbp_prey (cast `/Game/Blueprints/Character/BP_Prey` SenseActor))
  (`BlackboardComponent.SetValueAsObject` (`self.Blackboard`) "TargetActor" (select `bool` _bsuccessfullysensed :`true` _asbp_prey :!type "Object Object Reference"))
  (if (not _bsuccessfullysensed)
    (`BlackboardComponent.SetValueAsVector` (`self.Blackboard`) "LastLocation" _stimuluslocation)))

(fn `UserConstructionScript`
  (`parent.UserConstructionScript`))