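; AI controller for prey that uses sight perception to track predators and grass.
; Perception updates from sight feed HandleSightSense, which stores the seen predator or grass, or clears it and records the last known location when sight is lost.
; Only one reference is kept per type, and acting on this data is not handled here.
; A Testing flag makes Tick move the prey toward the player pawn.
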(event `self.ReceiveBeginPlay`
  (`parent.ReceiveBeginPlay`))

(event `self.ReceiveTick`
  (params (DeltaSeconds :type "Float (single-precision)"))
  (`parent.ReceiveTick` DeltaSeconds)
  (if (`self.testing`)
    (`self.MoveToActor` (`GameplayStatics.GetPlayerPawn` 0) -1.0 true true true null)))

(event `self.AIPerception.OnTargetPerceptionUpdated`
  (params (Actor :type "Actor Object Reference") (Stimulus :type "AIStimulus Structure"))
  (bind _returnvalue (`AIPerceptionSystem.GetSenseClassForStimulus` Stimulus))
  (if (== _returnvalue "/Script/AIModule.AISense_Sight")
    (`self.HandleSightSense` Actor Stimulus)))

(fn `HandleSightSense`
  (params (SenseActor :type "Actor Object Reference") (Stimulus :type "AIStimulus Structure"))
  (bind (_age _expirationage _strength _stimuluslocation _receiverlocation _tag _bsuccessfullysensed) (break `AIStimulus` Stimulus))
  (bind _asbp_predator (cast `/Game/Blueprints/Character/BP_Predator` SenseActor)
    (:`then`
      (if _bsuccessfullysensed
        (set `self.Predator` _asbp_predator)
        (else
          (set `self.Predator` null)
          (set `self.LastPredatorLocation` _stimuluslocation))))
    (:`CastFailed`
      (bind _asbp_grass (cast `/Game/Blueprints/Environment/BP_Grass` SenseActor))
      (if _bsuccessfullysensed
        (set `self.Grass` _asbp_grass)
        (else
          (set `self.Grass` null)
          (set `self.LastGrassLocation` _stimuluslocation))))))

(fn `UserConstructionScript`
  (`parent.UserConstructionScript`))